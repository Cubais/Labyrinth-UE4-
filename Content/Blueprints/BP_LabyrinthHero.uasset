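; BP_LabyrinthHero is the player hero Blueprint, handling HUD setup, a dynamic crosshair and aiming down sights.
; BeginPlay creates the labyrinth HUD and crosshair widgets and adds them to the viewport, keeping a reference to the crosshair.
; Tick maps movement speed to crosshair spread through a clamped range, so faster movement widens it.
; Holding AimDownSights swaps the first-person camera for the ADS camera and sets IsAiming until release.
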(event `self.ReceiveBeginPlay`
  (bind _returnvalue (`|CreateWidget` "/Game/Blueprints/Labyrinth_HUD.Labyrinth_HUD_C"))
  (`UserWidget.AddToViewport` _returnvalue 0)
  (bind _returnvalue_2 (`|CreateWidget` "/Game/Blueprints/DynamicCrossHair.WBCrosshair_C"))
  (bind _output_get (set `self.spread_ref` _returnvalue_2))
  (`UserWidget.AddToViewport` _returnvalue_2 0)
  (`UserWidget.AddToViewport` _output_get 0))

(event `self.ReceiveTick`
  (params (DeltaSeconds :type "Float (single-precision)"))
  (set `/Game/Blueprints/DynamicCrossHair.crosshair_spread` (`KismetMathLibrary.MapRangeClamped` (`KismetMathLibrary.VSize` (`self.GetVelocity`)) 0.0 450.0 5.0 80.0) (`self.spread_ref`)))

(event `InputAction|AimDownSights`
  (params (Key :type "Key Structure"))
  (bind _adscamera (`self.ADSCamera`))
  (:`Pressed`
    (`ActorComponent.Deactivate` (`self.FPVCamera`))
    (`ActorComponent.Activate` _adscamera false)
    (set `self.IsAiming` true))
  (:`Released`
    (`ActorComponent.Deactivate` _adscamera)
    (`ActorComponent.Activate` (`self.FPVCamera`) false)
    (set `self.IsAiming` false)))

(fn `UserConstructionScript`)